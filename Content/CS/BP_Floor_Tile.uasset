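; BP_Floor_Tile is a floor tile that places zombie spawners and can turn the running player.
; On BeginPlay it drops one random spawn point and spawns BP_ZombieSpawner at the other three, flagging SpawnPoint2 and SpawnPoint3 as right-side.
; On turn tiles, Box overlap slows the player to walk speed while a timeline lerps controller yaw by CombineRotation, then restores run speed.
; GetAttachTransform exposes the Arrow's world transform as an attach point.
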(event OnComponentBeginOverlap(Box)
  (params (OverlappedComponent :type Primitive%20Component%20Object%20Reference) (OtherActor :type Actor%20Object%20Reference) (OtherComp :type Primitive%20Component%20Object%20Reference) (OtherBodyIndex :type Integer) (bFromSweep :type Boolean) (SweepResult :type Hit%20Result%20Structure%20%28by%20ref%29))
  (bind _as_bp_first_person_character (Variables|Default|GetAs%20BP%20First%20Person%20Character))
  (bind _asbp_first_person_character (Utilities|Casting|CastToBP_FirstPersonCharacter OtherActor))
  (if (Variables|Default|GetbTurnTile)
    (Variables|Default|SetCurrentRotation (Pawn|GetControlRotation (Pawn|GetController _asbp_first_person_character) :!class /Script/Engine.Controller))
    (Variables|Default|SetTargetRotation (Math|Rotator|CombineRotators (Pawn|GetControlRotation (Pawn|GetController _asbp_first_person_character) :!class /Script/Engine.Controller) (Variables|Default|GetCombineRotation)))
    (Variables|Default|SetCurrentLocation (Transformation|GetActorLocation))
    (Default|SetWalkSpeed _as_bp_first_person_character)
    (bind _turnlerp (Timeline|Trun PlayFromStart)
      (:Update
        (Pawn|SetControlRotation (Pawn|GetController _asbp_first_person_character) (Math|Rotator|MakeRotator 0.0 0.0 (.yaw (Math|Rotator|Lerp(Rotator) (Variables|Default|GetCurrentRotation) (Variables|Default|GetTargetRotation) _turnlerp)))))
      (:Finished
        (Default|SetRunSpeed _as_bp_first_person_character)))))

(event EventBeginPlay
  (bind _spawnpointarr (Variables|Default|GetSpawnPointArr))
  (bind _asbp_first_person_character (Utilities|Casting|CastToBP_FirstPersonCharacter (Game|GetPlayerCharacter 0)))
  (Variables|Default|SetAs%20BP%20First%20Person%20Character _asbp_first_person_character)
  (Utilities|Array|RemoveItem _spawnpointarr (.OutItem (Utilities|Array|Random _spawnpointarr)))
  (for _array_element _spawnpointarr
    (if (or (== (Variables|Default|GetSpawnPoint2) _array_element) (== (Variables|Default|GetSpawnPoint3) _array_element))
      (Game|SpawnActorfromClass "/Game/YS/Blueprint/BP_ZombieSpawner.BP_ZombieSpawner_C" (Math|Conversions|ToTransform(Vector) (Transformation|GetWorldLocation _array_element)) "Undefined" "MultiplyWithRoot" 0 true 0)
      (else
        (Game|SpawnActorfromClass "/Game/YS/Blueprint/BP_ZombieSpawner.BP_ZombieSpawner_C" (Math|Conversions|ToTransform(Vector) (Transformation|GetWorldLocation _array_element)) "Undefined" "MultiplyWithRoot" 0 0)))))

(event Collision|EventActorBeginOverlap
  (params (OtherActor :type Actor%20Object%20Reference)))

(fn ConstructionScript
  (Variables|Default|SetSpawnPointArr (Utilities|Array|MakeArray (Variables|Default|GetSpawnPoint2) (Variables|Default|GetSpawnPoint1) (Variables|Default|GetSpawnPoint) (Variables|Default|GetSpawnPoint3))))

(fn GetAttachTransform
  (return (Transformation|GetWorldTransform (Variables|Default|GetArrow))))