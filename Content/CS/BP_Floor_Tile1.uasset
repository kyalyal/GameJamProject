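; BP_Floor_Tile1 is a floor tile for a zombie runner that chains via its NextArrow transform.
; On BeginPlay, turn tiles spawn a power skill item; others drop one random spawn point and place zombie spawners, flagged left or right.
; On turn tiles, a one-shot overlap timeline rotates and centers the player at walk speed, then restores running.
; Another overlap asks BP_ZombieGameMode for the next tile, then destroys this one after a delay.
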(event OnComponentBeginOverlap(TrunCollision)
  (params (OverlappedComponent :type Primitive%20Component%20Object%20Reference) (OtherActor :type Actor%20Object%20Reference) (OtherComp :type Primitive%20Component%20Object%20Reference) (OtherBodyIndex :type Integer) (bFromSweep :type Boolean) (SweepResult :type Hit%20Result%20Structure%20%28by%20ref%29))
  (bind _returnvalue (Transformation|GetActorLocation))
  (bind _as_bp_first_person_character (Variables|Default|GetAs%20BP%20First%20Person%20Character))
  (bind _as_bp_first_person_character_2 (Variables|Default|GetAs%20BP%20First%20Person%20Character))
  (bind _returnvalue_2 (Transformation|GetActorRotation _as_bp_first_person_character_2))
  ;[1 1 1] 코너회전
  (Utilities|Casting|CastToBP_FirstPersonCharacter OtherActor)
  (if (Variables|Default|GetbTurnTile)
    (Utilities|FlowControl|DoOnce false
      (:Completed
        (Variables|Default|SetCurrentRotation _returnvalue_2)
        (Variables|Default|SetTargetRotation (Math|Rotator|CombineRotators _returnvalue_2 (Variables|Default|GetCombineRotation)))
        (Variables|Default|SetCurrentPlayerLocation (Transformation|GetActorLocation (Game|GetPlayerCharacter 0)))
        (Default|SetWalkSpeed _as_bp_first_person_character)
        (bind _turnlerp (Timeline|Trun PlayFromStart)
          (:Update
            (Transformation|SetActorRotation (Variables|Default|GetAs%20BP%20First%20Person%20Character) (Math|Rotator|MakeRotator 0.0 0.0 (.yaw (Math|Rotator|Lerp(Rotator) (Variables|Default|GetCurrentRotation) (Variables|Default|GetTargetRotation) _turnlerp true))))
            (Transformation|SetActorLocation (Variables|Default|GetAs%20BP%20First%20Person%20Character) (Math|Vector|Lerp(Vector) (Variables|Default|GetCurrentPlayerLocation) (Math|Vector|MakeVector (.x _returnvalue) (.y _returnvalue) (.z (Variables|Default|GetCurrentPlayerLocation))) _turnlerp) false false))
          (:Finished
            (Default|SetRunSpeed _as_bp_first_person_character)))))))

(event OnComponentBeginOverlap(SpawnCollision)
  (params (OverlappedComponent :type Primitive%20Component%20Object%20Reference) (OtherActor :type Actor%20Object%20Reference) (OtherComp :type Primitive%20Component%20Object%20Reference) (OtherBodyIndex :type Integer) (bFromSweep :type Boolean) (SweepResult :type Hit%20Result%20Structure%20%28by%20ref%29))
  ;[1 1 1] 다음 타일 스폰
  (Utilities|Casting|CastToBP_FirstPersonCharacter OtherActor)
  (bind _asbp_zombie_game_mode (Utilities|Casting|CastToBP_ZombieGameMode (Game|GetGameMode)))
  (Utilities|FlowControl|DoOnce false
    (:Completed
      (Default|AddFloorTile _asbp_zombie_game_mode)
      (Utilities|FlowControl|Delay 2.0)
      (Actor|DestroyActor))))

(event EventBeginPlay
  (bind _spawnpointarr (Variables|Default|GetSpawnPointArr))
  (bind _asbp_first_person_character (Utilities|Casting|CastToBP_FirstPersonCharacter (Game|GetPlayerCharacter 0)))
  (Variables|Default|SetAs%20BP%20First%20Person%20Character _asbp_first_person_character)
  (if (Variables|Default|GetbTurnTile)
    ;[1 1 1] 코너 아이템 스폰
    (Game|SpawnActorfromClass "/Game/YS/Blueprint/Item/BP_PowerSkillItem.BP_PowerSkillItem_C" (Math|Transform|MakeTransform (Transformation|GetWorldLocation (Variables|Default|GetItemSpawnPoint)) "0, 0, 0" "1.000000,1.000000,1.000000") "Undefined" "MultiplyWithRoot" 0 0)
    (else
      (Utilities|Array|RemoveItem _spawnpointarr (.OutItem (Utilities|Array|Random _spawnpointarr)))
      (for _array_element _spawnpointarr
        (if (or (== (Variables|Default|GetSpawnPoint2) _array_element) (== (Variables|Default|GetSpawnPoint3) _array_element))
          ;[1 1 1] 오른쪽일 경우
          (Game|SpawnActorfromClass "/Game/YS/Blueprint/Zombie/BP_ZombieSpawner.BP_ZombieSpawner_C" (Transformation|GetWorldTransform _array_element) "Undefined" "MultiplyWithRoot" 0 true 0)
          (else
            ;[1 1 1] 왼쪽일 경우
            (Game|SpawnActorfromClass "/Game/YS/Blueprint/Zombie/BP_ZombieSpawner.BP_ZombieSpawner_C" (Transformation|GetWorldTransform _array_element) "Undefined" "MultiplyWithRoot" 0 false 0)))))))

(event Collision|EventActorBeginOverlap
  (params (OtherActor :type Actor%20Object%20Reference)))

(fn ConstructionScript
  (Variables|Default|SetSpawnPointArr (Utilities|Array|MakeArray (Variables|Default|GetSpawnPoint2) (Variables|Default|GetSpawnPoint1) (Variables|Default|GetSpawnPoint) (Variables|Default|GetSpawnPoint3))))

(fn GetAttachTransform
  (return (Transformation|GetWorldTransform (Variables|Default|GetNextArrow))))