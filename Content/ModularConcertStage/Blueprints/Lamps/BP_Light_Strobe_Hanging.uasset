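; Hanging strobe lamp prop for a modular concert stage, assembled procedurally in the construction script from a configurable number of stacked modules.
; Each module adds a strobe mesh and two side-by-side spot lights on the arm, spaced evenly downward, with the arm's yaw set by a rotation variable.
; Shared color and intensity variables drive the lights and a per-mesh dynamic emissive material, with volumetric beam strength set separately.
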(event EventBeginPlay)

(event Collision|EventActorBeginOverlap
  (params (OtherActor :type Actor%20Object%20Reference)))

(event EventTick
  (params (DeltaSeconds :type Float%20%28single-precision%29)))

(fn ConstructionScript
  (bind _light_intensity (Variables|Default|GetLight_Intensity))
  (bind _sm_strobe_arm (Variables|Default|GetSM_Strobe_Arm))
  (bind _light_color (Variables|Default|GetLight_Color))
  ;[1 1 1] Rotation
  (Transformation|SetRelativeRotation (Variables|Default|GetSM_Strobe_Arm) (Math|Rotator|MakeRotator 0.0 0.0 (Variables|Default|GetVertical_Rotation)) false false)
  (for _index (range 0 (- (Variables|Default|GetHow%20many?) 1))
    ;[1 1 1] Mesh Creation
    (bind _returnvalue (AddComponent|AddStaticMeshComponent false (Math|Transform|MakeTransform (Math|Vector|MakeVector 0.0 0.0 (+ (* (Math|Conversions|ToFloat(Integer) _index) -2e+01) -21.0)))))
    (Transformation|AttachComponentToComponent _returnvalue (Variables|Default|GetSM_Strobe_Arm) "None" "KeepRelative" "KeepRelative" "KeepRelative" true)
    (Components|StaticMesh|SetStaticMesh _returnvalue "/Game/ModularConcertStage/Meshes/Lamps_Parts/Strobe/SM_Storbe_Base.SM_Storbe_Base")
    ;[1 1 1] Light Creation
    (bind _returnvalue_2 (AddComponent|AddSpotLightComponent false (Math|Transform|MakeTransform (Math|Vector|MakeVector 8.0 -1e+01 (.z (Math|Vector|MakeVector 0.0 0.0 (+ (* (Math|Conversions|ToFloat(Integer) _index) -2e+01) -21.0)))))))
    ;[1 1 1] Attach
    (Transformation|AttachComponentToComponent _returnvalue_2 _sm_strobe_arm "None" "KeepRelative" "KeepRelative" "KeepRelative" true)
    (bind _returnvalue_3 (AddComponent|AddSpotLightComponent false (Math|Transform|MakeTransform (Math|Vector|MakeVector 8.0 1e+01 (.z (Math|Vector|MakeVector 0.0 0.0 (+ (* (Math|Conversions|ToFloat(Integer) _index) -2e+01) -21.0)))))))
    (Transformation|AttachComponentToComponent _returnvalue_3 _sm_strobe_arm "None" "KeepRelative" "KeepRelative" "KeepRelative" true)
    ;[1 1 1] Set Light Properties
    (bind _returnvalue_4 (Rendering|Material|CreateDynamicMaterialInstance _returnvalue 1 "/Game/ModularConcertStage/Materials/Instances/MI_Light_Emissive_Strobe.MI_Light_Emissive_Strobe" "None" :!class /Script/Engine.PrimitiveComponent))
    (Rendering|Material|SetVectorParameterValue _returnvalue_4 "Light_Color" _light_color :!class /Script/Engine.MaterialInstanceDynamic)
    (Rendering|Material|SetScalarParameterValue _returnvalue_4 "Light_Emissive_Intensity" (/ _light_intensity 1e+03) :!class /Script/Engine.MaterialInstanceDynamic)
    (Rendering|Components|Light|SetLightColor _returnvalue_2 _light_color true)
    (Rendering|Components|Light|SetIntensity _returnvalue_3 _light_intensity)
    (Class|LightComponent|SetVolumetricScatteringIntensity _returnvalue_3 (Variables|Default|GetLight%20Beam%20Intensity))))