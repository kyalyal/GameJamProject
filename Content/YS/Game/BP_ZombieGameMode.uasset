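; BP_ZombieGameMode is a game mode that builds a procedural floor path from chained tiles, laying an initial run at BeginPlay.
; AddFloorTile spawns a random straight tile class and counts straights, handing off to AddFloorCurve for a random curve once eight are placed, which resets the count.
; Each spawned BP_Floor_Tile supplies its attach transform as the next spawn point, so pieces connect end to end.
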(event EventBeginPlay
  (for _index (range 0 9)
    (CallFunction|AddFloorTile)))

(event EventTick
  (params (DeltaSeconds :type Float%20%28single-precision%29)))

(fn ConstructionScript)

(fn AddFloorTile
  (bind _floortiles (Variables|Default|GetFloorTiles))
  (if (> (Variables|Default|GetCurrentStraights) 7)
    (CallFunction|AddFloorCurve)
    (else
      (bind _returnvalue (Game|SpawnActorfromClass (Utilities|Array|Get(acopy) _floortiles (Math|Random|RandomIntegerinRange 0 (Utilities|Array|LastIndex _floortiles))) (Variables|Default|GetNextSpawnPoint) "Undefined" "MultiplyWithRoot" 0 0))
      (bind _asbp_floor_tile (Utilities|Casting|CastToBP_Floor_Tile _returnvalue))
      (bind _attachtransform (Default|GetAttachTransform _asbp_floor_tile))
      (Variables|Default|SetNextSpawnPoint _attachtransform)
      (Variables|Default|SetCurrentStraights (+ (Variables|Default|GetCurrentStraights) 1)))))

(fn AddFloorCurve
  (bind _floorcurves (Variables|Default|GetFloorCurves))
  (bind _returnvalue (Game|SpawnActorfromClass (Utilities|Array|Get(acopy) _floorcurves (Math|Random|RandomIntegerinRange 0 (Utilities|Array|LastIndex _floorcurves))) (Variables|Default|GetNextSpawnPoint) "Undefined" "MultiplyWithRoot" 0 0))
  (bind _asbp_floor_tile (Utilities|Casting|CastToBP_Floor_Tile _returnvalue))
  (bind _attachtransform (Default|GetAttachTransform _asbp_floor_tile))
  (Variables|Default|SetNextSpawnPoint _attachtransform)
  (Variables|Default|SetCurrentStraights 0))