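; BP_PowerSkillItem is a syringe pickup actor that heals the first-person character on contact, despite its power-skill name.
; Its sphere overlap casts the other actor to BP_FirstPersonCharacter and calls Heal with a fixed amount.
; It then calls ChangeSkeletalItem on the character with the syringe mesh, push animation and hands montage, and destroys itself.
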(event OnComponentBeginOverlap(Sphere)
  (params (OverlappedComponent :type Primitive%20Component%20Object%20Reference) (OtherActor :type Actor%20Object%20Reference) (OtherComp :type Primitive%20Component%20Object%20Reference) (OtherBodyIndex :type Integer) (bFromSweep :type Boolean) (SweepResult :type Hit%20Result%20Structure%20%28by%20ref%29))
  (bind _asbp_first_person_character (Utilities|Casting|CastToBP_FirstPersonCharacter OtherActor))
  (Default|Heal _asbp_first_person_character 1e+02)
  (Default|ChangeSkeletalItem _asbp_first_person_character "/Game/FPS_Starter_Pack/Animations/Syringe_03/Anim_Syringe_03_Push.Anim_Syringe_03_Push" "/Game/FPS_Starter_Pack/Animations/Syringe_03/Anim_Hands_Syringe_03_Using_Montage.Anim_Hands_Syringe_03_Using_Montage" "/Game/FPS_Starter_Pack/Mesh/SK_Stuff/SK_Syringe_03.SK_Syringe_03")
  (Actor|DestroyActor))

(event EventBeginPlay
  (|CallParentFunction) ; 지금 이 노드는 비활성 상태입니다. \n핀을 끌어서 다른 노드를 연결하면 활성화됩니다.
)

(event Collision|EventActorBeginOverlap
  (params (OtherActor :type Actor%20Object%20Reference))
  (|CallParentFunction OtherActor) ; 지금 이 노드는 비활성 상태입니다. \n핀을 끌어서 다른 노드를 연결하면 활성화됩니다.
)

(event EventTick
  (params (DeltaSeconds :type Float%20%28single-precision%29))
  (|CallParentFunction DeltaSeconds) ; 지금 이 노드는 비활성 상태입니다. \n핀을 끌어서 다른 노드를 연결하면 활성화됩니다.
)

(fn ConstructionScript
  (|CallParentFunction))