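; BP_ZombieW is a zombie actor that the first-person player can knock down with an attack in the matching direction.
; When the player overlaps its Box while attacking and the attack direction matches the zombie's IsRight flag, a Niagara blood burst spawns at the left or right blood point.
; The skeletal mesh then switches to physics and is launched along the player's forward vector.
; InPlayer tracks whether the player is inside the Box.
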(event OnComponentBeginOverlap(Box)
  (params (OverlappedComponent :type Primitive%20Component%20Object%20Reference) (OtherActor :type Actor%20Object%20Reference) (OtherComp :type Primitive%20Component%20Object%20Reference) (OtherBodyIndex :type Integer) (bFromSweep :type Boolean) (SweepResult :type Hit%20Result%20Structure%20%28by%20ref%29))
  (bind _asbp_first_person_character (Utilities|Casting|CastToBP_FirstPersonCharacter OtherActor))
  (Variables|Default|SetInPlayer true)
  (if (Variables|/Game/YS/Character/BP_FirstPersonCharacter.BP_FirstPersonCharacter_C|GetbIsAttack _asbp_first_person_character)
    (if (== (Variables|/Game/YS/Character/BP_FirstPersonCharacter.BP_FirstPersonCharacter_C|GetDir _asbp_first_person_character) (Variables|Default|GetbIsRight))
      (if (Variables|Default|GetbIsRight)
        (Niagara|SpawnSystematLocation "/Game/Vefects/Blood_VFX/VFX/VAT_Versions/Bursts/Looped/Looped_NS_HD_Blood_Burst_Large_Orange.Looped_NS_HD_Blood_Burst_Large_Orange" (Transformation|GetWorldLocation (Variables|Default|GetRightBlood)) "0, 0, 0" "5.000000,5.000000,5.000000")
        (else
          (Niagara|SpawnSystematLocation "/Game/Vefects/Blood_VFX/VFX/VAT_Versions/Bursts/Looped/Looped_NS_HD_Blood_Burst_Large_Orange.Looped_NS_HD_Blood_Burst_Large_Orange" (Transformation|GetWorldLocation (Variables|Default|GetLeftBlood)) "0, 0, 0" "5.000000,5.000000,5.000000")))
      (Physics|SetSimulatePhysics (Variables|Default|GetSkeletalMesh) true)
      (Physics|AddForce (Variables|Default|GetSkeletalMesh) (* (Transformation|GetActorForwardVector (Game|GetPlayerCharacter 0)) 5e+06) "None" false))))

(event OnComponentEndOverlap(Box)
  (params (OverlappedComponent :type Primitive%20Component%20Object%20Reference) (OtherActor :type Actor%20Object%20Reference) (OtherComp :type Primitive%20Component%20Object%20Reference) (OtherBodyIndex :type Integer))
  (Utilities|Casting|CastToBP_FirstPersonCharacter OtherActor)
  (Variables|Default|SetInPlayer false))

(event EventBeginPlay)

(event Collision|EventActorBeginOverlap
  (params (OtherActor :type Actor%20Object%20Reference)))

(event EventTick
  (params (DeltaSeconds :type Float%20%28single-precision%29)))

(fn ConstructionScript)