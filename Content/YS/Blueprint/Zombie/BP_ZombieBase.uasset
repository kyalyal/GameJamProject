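; Base Blueprint for zombies that the first-person player can kill by attacking on the matching side.
; When the player enters the Box trigger, a one-time kill fires if they are already attacking and their Dir matches IsRight.
; The kill spawns a Niagara blood burst, then ragdolls the mesh along the player's forward vector with a hit sound before delayed destruction.
; When the player leaves the trigger, the zombie is also destroyed after a short delay.
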(event OnComponentBeginOverlap(Box)
  (params (OverlappedComponent :type Primitive%20Component%20Object%20Reference) (OtherActor :type Actor%20Object%20Reference) (OtherComp :type Primitive%20Component%20Object%20Reference) (OtherBodyIndex :type Integer) (bFromSweep :type Boolean) (SweepResult :type Hit%20Result%20Structure%20%28by%20ref%29))
  (bind _asbp_first_person_character (Utilities|Casting|CastToBP_FirstPersonCharacter OtherActor))
  (Variables|Default|SetInPlayer true)
  (if (Variables|/Game/YS/Character/BP_FirstPersonCharacter.BP_FirstPersonCharacter_C|GetbIsAttack _asbp_first_person_character)
    (if (== (Variables|/Game/YS/Character/BP_FirstPersonCharacter.BP_FirstPersonCharacter_C|GetDir _asbp_first_person_character) (Variables|Default|GetbIsRight))
      (Utilities|FlowControl|DoOnce false
        (:Completed
          (Niagara|SpawnSystematLocation "/Game/Vefects/Blood_VFX/VFX/VAT_Versions/Bursts/Looped/Looped_NS_HD_Blood_Burst_Large_Orange.Looped_NS_HD_Blood_Burst_Large_Orange" (Transformation|GetWorldLocation (Variables|Default|GetBloodSpawnPoint)) "0, 0, 0" "5.000000,5.000000,5.000000")
          (CallFunction|Death))))))

(event OnComponentEndOverlap(Box)
  (params (OverlappedComponent :type Primitive%20Component%20Object%20Reference) (OtherActor :type Actor%20Object%20Reference) (OtherComp :type Primitive%20Component%20Object%20Reference) (OtherBodyIndex :type Integer))
  (Utilities|Casting|CastToBP_FirstPersonCharacter OtherActor)
  (Variables|Default|SetInPlayer false)
  (Utilities|FlowControl|Delay 3.0)
  (Actor|DestroyActor))

(event Custom|Death
  ;[1 1 1] 죽음처리
  (Physics|SetSimulatePhysics (Variables|Default|GetSkeletalMesh) true)
  (Physics|AddForce (Variables|Default|GetSkeletalMesh) (* (Transformation|GetActorForwardVector (Game|GetPlayerCharacter 0)) 5e+06) "None" false)
  (Audio|SpawnSoundatLocation "/Game/Sword_Fighting_SFX/Wavs/RandomZombieHitBlunt_Weapon_Hits_Flesh_1_Cue.RandomZombieHitBlunt_Weapon_Hits_Flesh_1_Cue" (Transformation|GetActorLocation) "0, 0, 0" 1.0 1.0 0.0 0 0)
  (Utilities|FlowControl|Delay 5.0)
  (Actor|DestroyActor)
  (Actor|DestroyActor))

(event EventBeginPlay)

(event Collision|EventActorBeginOverlap
  (params (OtherActor :type Actor%20Object%20Reference)))

(event EventTick
  (params (DeltaSeconds :type Float%20%28single-precision%29)))

(fn ConstructionScript)