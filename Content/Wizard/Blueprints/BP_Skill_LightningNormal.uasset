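; BP_Skill_LightningNormal is a wizard lightning skill actor that kills zombies around the point where it spawns.
; On BeginPlay it spawns an intro effect, then the main lightning effect after a short delay.
; A second delay precedes a multi-sphere trace on the Visibility channel around the actor.
; Each hit actor that casts to BP_ZombieBase has Death called directly, with no damage calculation.
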(event EventBeginPlay
  (Niagara|SpawnSystematLocation "/Game/Wizard/Particles/Lightning/PS_Lightning_Intro.PS_Lightning_Intro" (Transformation|GetActorLocation self))
  (Utilities|FlowControl|Delay 0.9)
  (Niagara|SpawnSystematLocation "/Game/Wizard/Particles/Lightning/PS_Lightning_Classic_a.PS_Lightning_Classic_a" (Transformation|GetActorLocation self))
  (Utilities|FlowControl|Delay 0.5)
  (bind _outhits (Collision|MultiSphereTraceByChannel (Transformation|GetActorLocation) "0, 0, 0" 5e+02 "TraceTypeQuery1" false 0 "None"))
  (for _array_element _outhits
    (bind _asbp_zombie_base (Utilities|Casting|CastToBP_ZombieBase (.HitActor (Collision|BreakHitResult _array_element))))
    (Default|Death _asbp_zombie_base)))

(fn ConstructionScript)